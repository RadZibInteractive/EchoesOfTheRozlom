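; Shooter pickup Blueprint that animates its mesh while idle and when it respawns.
; Tick calls Spin, which uses game time to yaw the mesh steadily and bob it on a sine wave, setting unit scale each frame.
; OnRespawn plays a timeline that drives mesh scale, then calls FinishRespawn, which is defined outside this graph.
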(event EventOnRespawn
  (bind _scale (Timeline|Respawn PlayFromStart)
    (:Update
      (Transformation|SetRelativeScale3D (Variables|Character|GetMesh) (Math|Conversions|ToVector(Float) _scale)))
    (:Finished
      (Class|EotRPickup|FinishRespawn))))

(event EventTick
  (params (DeltaSeconds :type Float%20%28single-precision%29))
  (CallFunction|Spin "1.000000,1.000000,1.000000"))

(fn ConstructionScript)

(fn Spin
  (params (New%20Transform%20Scale :type Vector :default "1.000000,1.000000,1.000000"))
  (bind _returnvalue (Utilities|Time|GetGameTimeinSeconds))
  (Transformation|SetRelativeTransform (Variables|Character|GetMesh) (Math|Transform|MakeTransform (Math|Vector|MakeVector 0.0 0.0 (* (Math|Trig|Sin(Radians) (* _returnvalue 3.0)) 15.0)) (Math|Rotator|MakeRotator 0.0 0.0 (* _returnvalue 1e+02)) New%20Transform%20Scale) false false))